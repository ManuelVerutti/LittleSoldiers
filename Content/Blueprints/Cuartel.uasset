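; Barracks Blueprint for a clicker-style game that earns coins from taps on the base and spawns units.
; On BeginPlay it adds GameUI and starts a looping SummonSoldier timer, which ActualizateTimer restarts using SummonSpeed.
; Touch and mouse traces hitting an actor tagged "Base" add CoinsClick to Coins, and Tick refreshes the coin text every frame.
; SummonCar alternates between two offset spawn positions but is not called within this graph.
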(event Custom|Summon
  (CallFunction|SummonSoldier))

(event Custom|ActualizateTimer
  (Utilities|Time|SetTimerbyEvent (delegate Custom|Summon) (Variables|Default|GetSummonSpeed) true))

(event EventBeginPlay
  (bind _returnvalue (Game|ConstructObjectfromClass "/Game/GUI/GameUI.GameUI_C"))
  (UserInterface|Viewport|AddtoViewport _returnvalue 0)
  (Utilities|Time|SetTimerbyEvent (delegate Custom|Summon) (Variables|Default|GetSummonSpeed) true))

(event Collision|EventActorBeginOverlap
  (params (OtherActor :type Actor%20Object%20Reference)))

(event MouseInput|EventActorOnClicked
  (params (ButtonPressed :type Key%20Structure :default "None")))

(event EventTick
  (params (DeltaSeconds :type Float%20%28single-precision%29))
  (Class|Text3DComponent|SetText (Variables|Default|GetUiCoins) (Utilities|Text|ToText(Float) (stale Input|MouseEvents|LeftMouseButton _output_get) "HalfToEven")))

(event Input|MouseEvents|LeftMouseButton
  (params (Key :type Key%20Structure :default "None"))
  (bind _returnvalue (Game|GetPlayerController 0))
  (bind (_worldlocation _worlddirection) (Game|Player|ConvertMouseLocationToWorldSpace _returnvalue))
  (:Pressed
    (bind _outhit (Collision|LineTraceByChannel _worldlocation (+ _worldlocation (* _worlddirection 1e+08)) "TraceTypeQuery1" false 0 "None"))
    (if (Actor|ActorHasTag (.HitActor (Collision|BreakHitResult _outhit)) "Base")
      (bind _output_get (Variables|Default|SetCoins (+ (Variables|Default|GetCoins) (Variables|Default|GetCoinsClick))))
      (Class|Text3DComponent|SetText (Variables|Default|GetUiCoins) (Utilities|Text|ToText(Float) _output_get "HalfToEven")))))

(event Input|TouchEvents|InputTouch
  (params (Location :type Vector) (FingerIndex :type ETouchIndex%20Enum))
  (:Pressed
    (if (Actor|ActorHasTag (.HitActor (Collision|BreakHitResult (.HitResult (Class|PlayerController|GetHitResultUnderFingerbyChannel (Game|GetPlayerController 0) "Touch1" "TraceTypeQuery2" true)))) "Base")
      (bind _output_get (Variables|Default|SetCoins (+ (Variables|Default|GetCoins) (Variables|Default|GetCoinsClick))))
      (Class|Text3DComponent|SetText (Variables|Default|GetUiCoins) (Utilities|Text|ToText(Float) _output_get "HalfToEven")))))

(fn ConstructionScript)

(fn SummonSoldier
  (Game|SpawnActorfromClass "/Game/Blueprints/GreenArmy/Soldier.Soldier_C" (Math|Conversions|ToTransform(Vector) (Variables|Default|GetSummonPositionSoldier)) "Undefined" 0 0))

(fn SummonCar
  (bind _summonpositioncar (Variables|Default|GetSummonPositionCar))
  (if (Variables|Default|GetLastCarSummonedPosLeft)
    (Variables|Default|SetLastCarSummonedPosLeft false)
    (Game|SpawnActorfromClass "/Game/Blueprints/GreenArmy/Car.Car_C" (Math|Conversions|ToTransform(Vector) (+ _summonpositioncar "600.000000,0.000000,0")) "Undefined" 0 0)
    (else
      (Variables|Default|SetLastCarSummonedPosLeft true)
      (Game|SpawnActorfromClass "/Game/Blueprints/GreenArmy/Car.Car_C" (Math|Conversions|ToTransform(Vector) _summonpositioncar) "Undefined" 0 0))))