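; Green army car character that drives itself to the nearest enemy base and cashes in coins for the player on arrival.
; A looping timer set at BeginPlay repeatedly gathers actors tagged EnemyBase and issues an AI MoveTo toward the closest one.
; Overlapping a tagged base adds a fixed reward to Coins on the player's Cuartel pawn, then destroys the car.
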(event Custom|FindEnemy
  (bind _outactors (Actor|GetAllActorswithTag "EnemyBase"))
  (AI|AIMoveTo (Class|PawnMovementComponent|GetPawnOwner (Variables|Character|GetCharacterMovement)) "0, 0, 0" (.ReturnValue (Actor|FindNearestActor (Transformation|GetActorLocation) _outactors)) 5.0 false))

(event Collision|EventActorBeginOverlap
  (params (OtherActor :type Actor%20Object%20Reference))
  (if (Actor|ActorHasTag OtherActor "EnemyBase")
    (bind _ascuartel (Utilities|Casting|CastToCuartel (Game|Player|GetPlayerPawn 0)))
    (Variables|/Game/Blueprints/Cuartel.Cuartel_C|SetCoins _ascuartel (+ (Variables|/Game/Blueprints/Cuartel.Cuartel_C|GetCoins _ascuartel) 1.2e+04))
    (Actor|DestroyActor)))

(event EventBeginPlay
  (Utilities|Time|SetTimerbyEvent (delegate Custom|FindEnemy) 0.2 true))

(fn ConstructionScript)